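; Player controller for the networked metaverse, handling chat, character spawning, camera and session exit.
; On begin play it caches and hides the ChatHUD widgets and views a level CameraActor; messages are relayed through every PC_Metaverse.
; The GameInstance's chosen character spawns on the server at a PlayerStart, tagged "X" as taken, and is possessed with movement disabled.
; Kick and host-leave events destroy the session and reopen character selection.
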(event `self.ReceiveBeginPlay`
  ;[1 1 1] Begin | Check Local Controller | Visibility of Message Box and Player List
  (`|ExecutionSequence`
    (:`then_0`
      (if (`self.IsLocalController`)
        (`KismetSystemLibrary.Delay` 0.0)
        (bind _asbp_chat_hud (cast `/Game/Network/Widget/BP_ChatHUD` (`self.GetHUD`)))
        (bind _output_get (set `self.ChatHUD` _asbp_chat_hud))
        (`|ExecutionSequence`
          (:`then_0`
            (bind _output_get_2 (set `self.MessageBox_Ref` (`/Game/Network/Widget/BP_ChatHUD.MessageBox_Ref` _output_get)))
            (`Widget.SetVisibility` _output_get_2 "Hidden"))
          (:`then_1`
            (bind _output_get_3 (set `self.Player List Ref` (`/Game/Network/Widget/BP_ChatHUD.PlayerList_Ref` _output_get)))
            (`Widget.SetVisibility` _output_get_3 "Hidden")))))
    (:`then_1`
      (`self.SetCamera`))))

(event `AddMessage`
  (params (UserName :type Text) (Message :type Text))
  ;[1 1 1] Send Or Add Messages
  (`/Game/Network/Widget/WBP_MessageBox.AddMessage` (`self.MessageBox_Ref`) UserName Message))

(event `SendMessage`
  (params (UserName :type Text) (Message :type Text))
  ;[1 1 1] Send Or Add Messages
  (bind _outactors (`GameplayStatics.GetAllActorsOfClass` "PC_Metaverse_C"))
  (for _array_element _outactors
    (`/Engine/EditorBlueprintResources/StandardMacros.IsValid` _array_element
      (:`Is Valid`
        (`self.AddMessage` _array_element UserName Message)))))

(event `Client_SpawnPlayer`
  ;[1 1 1] OwingClient
  (bind _asgi_metaverse (cast `/Game/Network/Core/GI_Metaverse` (`GameplayStatics.GetGameInstance`)))
  (`self.Server_SpawnPlayer` (`/Game/Network/Core/GI_Metaverse.Character` _asgi_metaverse)))

(event `OwingClient_KickPlayer`
  ;[1 1 1] Kick Player
  (`DestroySessionCallbackProxy.DestroySession` (`GameplayStatics.GetPlayerController` 0)
    (:`OnSuccess`
      (`GameplayStatics.OpenLevelBySoftObjectPtr` "/Game/Network/Map/Level_CharacterSelection.Level_CharacterSelection" true "listen"))))

(event `EndSessionByServer`
  ;[1 1 1] Host Destroy The Session (Used In Leave Session in WBP_MainUI)
  (`DestroySessionCallbackProxy.DestroySession` self
    (:`OnSuccess`
      (`GameplayStatics.OpenLevelBySoftObjectPtr` "/Game/Network/Map/Level_CharacterSelection.Level_CharacterSelection" true "listen"))))

(event `Server_SpawnPlayer`
  (params (Class :type "Actor Class Reference"))
  ;[1 1 1] Server
  (bind _outactors (`GameplayStatics.GetAllActorsOfClass` "/Script/Engine.PlayerStart"))
  (for _array_element _outactors
    (if (!= (`PlayerStart.PlayerStartTag` _array_element) "X")
      (set `PlayerStart.PlayerStartTag` "X" _array_element)
      (break)))
  (bind _returnvalue (`|SpawnActorFromClass` Class (`self.GetTransform` _array_element) "Undefined" "OverrideRootScale" null null))
  (bind _ascharacter (cast `Character` _returnvalue :!pure true))
  (`/Engine/EditorBlueprintResources/StandardMacros.IsValid` _ascharacter
    (:`Is Valid`
      (`CharacterMovementComponent.DisableMovement` (`Character.CharacterMovement` _ascharacter))
      (`self.Possess` _ascharacter))))

(event `SetCamera`
  ;[1 1 1] Set Camera View
  (bind _returnvalue (`GameplayStatics.GetActorOfClass` "/Script/Engine.CameraActor"))
  (`self.SetViewTargetWithBlend` _returnvalue))

(fn `UserConstructionScript`)