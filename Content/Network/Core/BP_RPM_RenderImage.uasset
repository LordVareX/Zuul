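; BP_RPM_RenderImage is an image widget that displays an RPM render loaded from a URL.
; LoadImage spawns a BP_RPM_RenderActor far below the world origin and tells it to load the render with the given URL and capture animation.
; When the actor's OnCaptured event fires, the widget sets the resulting material as its brush and becomes visible.
; OnDestroy destroys the render actor.
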(event `LoadImage`
  ;[1 1 1] Spawn render actor
  (bind _returnvalue (`|SpawnActorFromClass` "/Game/Network/Core/BP_RPM_RenderActor.BP_RPM_RenderActor_C" (`KismetMathLibrary.MakeTransform` (0.0 0.0 -30000.0) (struct :`Roll` -90.0)) "Undefined" "OverrideRootScale" null null))
  (bind _output_get (set `self.RenderActor` _returnvalue))
  ;[1 1 1] Load render and display the image
  (add `/Game/Network/Core/BP_RPM_RenderActor.OnCaptured` _output_get (delegate `ImageLoaded`))
  (`/Game/Network/Core/BP_RPM_RenderActor.LoadRender` _output_get (`self.CaptureAnimation`) (`self.Url`)))

(event `ImageLoaded`
  (params (NewParam :type "MaterialInstanceDynamic Object Reference"))
  ;[1 1 1] Load render and display the image
  (`self.SetBrushFromMaterial` NewParam)
  (`self.SetVisibility` "Visible"))

(event `On Destroy`
  (bind _renderactor (`self.RenderActor`))
  ;[1 1 1] Destroy the render actor
  (`/Engine/EditorBlueprintResources/StandardMacros.IsValid` _renderactor
    (:`Is Valid`
      (`Actor.K2_DestroyActor` _renderactor))))