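; GM_Metaverse is the game mode for a GameLift-hosted multiplayer metaverse server, handling session lifecycle and player management.
; On server start it initializes the GameLift SDK and reports the process ready on the server's port.
; Logins register controllers, refresh player-list widgets, trigger client spawning and set the camera; spawning uses a random PlayerStart.
; Logouts remove GameLift player sessions, shutting the process down when empty; players can also be kicked by index.
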(event `self.ReceiveBeginPlay`
  (bind _as_gi_metaverse (`self.As GI Metaverse`))
  ;[1 1 1] Initiate Connection to Gamelift
  (`parent.ReceiveBeginPlay`)
  (if (`KismetSystemLibrary.IsServer`)
    (bind _asgi_metaverse (cast `/Game/Network/Core/GI_Metaverse` (`GameplayStatics.GetGameInstance`)))
    (set `self.As GI Metaverse` _asgi_metaverse)
    (bind (_success _errortype _errormessage) (`GameLiftServerFunctionLibrary.InitSDK`))
    (if _success
      (bind _returnvalue (`|GenericCreateObject` :`self` _as_gi_metaverse :`Class` "/Game/Blueprints/MetaverseProcessParameter.MetaverseProcessParameter_C"))
      (set `ProcessParameters.port` (`.port` (`ServerHelper.ServerIPAndPort`)) _returnvalue)
      (bind _output_get (set `/Game/Network/Core/GI_Metaverse.ProcessParameter` _returnvalue _as_gi_metaverse))
      (bind (_success_2 _errortype_2 _errormessage_2) (`GameLiftServerFunctionLibrary.ProcessReady` _output_get))
      (if (not _success_2)
        (`KismetSystemLibrary.PrintString` _errormessage_2))
      (else
        (`KismetSystemLibrary.PrintString` _errormessage)))))

(event `self.K2_PostLogin`
  (params (NewPlayer :type "PlayerController Object Reference"))
  ;[1 1 1] When a player is connected (Must check all players)
  (bind _aspc_metaverse (cast `/Game/Network/Core/PC_Metaverse` NewPlayer))
  (set `self.PC Metaverse_Ref` _aspc_metaverse)
  (`|ExecutionSequence`
    (:`then_0`
      (`KismetArrayLibrary.Array_Add` (`self.AllPlayersController`) (`self.PC Metaverse_Ref`))
      ;[1 1 1] Access to Update Player List
      (`self.UpdatePlayerList`))
    (:`then_1`
      (`/Game/Network/Core/PC_Metaverse.Client_SpawnPlayer` (`self.PC Metaverse_Ref`)))
    (:`then_2`
      (`self.SetCamera`))))

(event `self.K2_OnSwapPlayerControllers`
  (params (OldPC :type "PlayerController Object Reference") (NewPC :type "PlayerController Object Reference"))
  ;[1 1 1] When a player is connected (Must check all players)
  (`KismetArrayLibrary.Array_Add` (`self.JoinPlayers`) NewPC))

(event `self.K2_OnLogout`
  (params (ExitingController :type "Controller Object Reference"))
  ;[1 1 1] When a player is disconnected
  (bind _aspc_metaverse (cast `/Game/Network/Core/PC_Metaverse` ExitingController))
  (`KismetArrayLibrary.Array_RemoveItem` (`self.AllPlayersController`) _aspc_metaverse)
  ;[1 1 1] Remove Player Session on Gamelift when Players quit
  (bind _asps_metaverse (cast `/Game/Network/Core/PS_Metaverse` (`Controller.PlayerState` ExitingController)))
  (bind (_success _errortype _errormessage) (`GameLiftServerFunctionLibrary.RemovePlayerSession` (`/Game/Network/Core/PS_Metaverse.PlayerSessionID` _asps_metaverse)))
  (if _success
    (`self.CloseGameSession`)
    (else
      (`KismetSystemLibrary.PrintString` _errormessage))))

(event `CloseGameSession`
  ;[1 1 1] Shut down Game Session if no player inside Game Session
  (if (== (`KismetArrayLibrary.Array_Length` (`self.AllPlayersController`)) 0)
    (bind (_success _errortype _errormessage) (`GameLiftServerFunctionLibrary.ProcessEnding`))
    (if _success
      (bind (_success_2 _errortype_2 _errormessage_2) (`GameLiftServerFunctionLibrary.Destroy`))
      (if (not _success_2)
        (`KismetSystemLibrary.PrintString` _errormessage_2))
      (else
        (`KismetSystemLibrary.PrintString` _errormessage)))
    (else
      (`self.UpdatePlayerList`))))

(event `UpdatePlayerList`
  ;[1 1 1] Update Player List (Game Mode)
  (`KismetSystemLibrary.Delay` 0.3)
  (bind _foundwidgets (`WidgetBlueprintLibrary.GetAllWidgetsOfClass` "/Game/Network/Widget/WBP_PlayerList.WBP_PlayerList_C" false))
  (for _array_element _foundwidgets
    (`/Game/Network/Widget/WBP_PlayerList.UpdateWidget` _array_element)))

(event `SetCamera`
  ;[1 1 1] Default Camera
  (bind _returnvalue (`GameplayStatics.GetActorOfClass` "/Script/Engine.CameraActor"))
  (`PlayerController.SetViewTargetWithBlend` (`self.PC Metaverse_Ref`) _returnvalue 0.0 "VTBlend_Linear" 0.0 false))

(fn `Find_Random_PlayerStart`
  (returns (PlayerStartTransform :type "Transform Structure"))
  (bind _outactors (`GameplayStatics.GetAllActorsOfClass` "/Script/Engine.PlayerStart"))
  (return (`self.GetTransform` (`|GetArrayItem` _outactors (`KismetMathLibrary.RandomIntegerInRange` 0 (- (`KismetArrayLibrary.Array_Length` _outactors) 1))))))

(fn `KickPlayer`
  (params (PlayerID :type Integer))
  (`/Game/Network/Core/PC_Metaverse.OwingClient_KickPlayer` (`|GetArrayItem` (`self.AllPlayersController`) PlayerID)))

(fn `Spawn_Player`
  (params (PlayerController :type "PlayerController Object Reference"))
  (bind _returnvalue (`Controller.K2_GetPawn` PlayerController))
  (`/Engine/EditorBlueprintResources/StandardMacros.IsValid` _returnvalue
    (:`Is Valid`
      (`self.K2_DestroyActor` _returnvalue))
    (:`Is Not Valid`
      _))
  (bind _returnvalue_2 (`|SpawnActorFromClass` (`/Game/Network/Core/GI_Metaverse.Character` (cast `/Game/Network/Core/GI_Metaverse` (`GameplayStatics.GetGameInstance`) :!pure true)) (`self.Find_Random_PlayerStart`) "Undefined" "OverrideRootScale" null null))
  (`Controller.Possess` PlayerController _returnvalue_2))

(fn `UserConstructionScript`)