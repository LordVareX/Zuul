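; Player controller for a multiplayer metaverse with avatars, chat and proximity-style voice.
; BeginPlay hides local chat widgets, views a level CameraActor and retries until it can register a VOIP talker attached to player character 0's capsule.
; The client sends its GameInstance avatar URL to the server, which claims a PlayerStart by tagging it "X", then spawns and possesses a movement-disabled pawn.
; Kick and host-leave events destroy the session and open character selection.
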(event `self.ReceiveBeginPlay`
  (bind _playerstate (`self.PlayerState`))
  (bind _asbp_parent (cast `/Game/TestCharacters/ParentMain/BP_Parent` (`GameplayStatics.GetPlayerCharacter` 0) :!pure true))
  ;[1 1 1] Begin | Check Local Controller | Visibility of Message Box and Player List
  (`|ExecutionSequence`
    (:`then_0`
      (if (`self.IsLocalController`)
        (`KismetSystemLibrary.Delay` 0.0)
        (bind _asbp_chat_hud (cast `/Game/Network/Widget/BP_ChatHUD` (`self.GetHUD`)))
        (bind _output_get (set `self.ChatHUD` _asbp_chat_hud))
        (`|ExecutionSequence`
          (:`then_0`
            (bind _output_get_2 (set `self.MessageBox_Ref` (`/Game/Network/Widget/BP_ChatHUD.MessageBox_Ref` _output_get)))
            (`Widget.SetVisibility` _output_get_2 "Hidden"))
          (:`then_1`
            (bind _output_get_3 (set `self.Player List Ref` (`/Game/Network/Widget/BP_ChatHUD.PlayerList_Ref` _output_get)))
            (`Widget.SetVisibility` _output_get_3 "Hidden")))))
    (:`then_1`
      (`self.SetCamera`))
    (:`then_2`
      (bind _returnvalue (`AddComponent|NODE_AddVOIPTalker-0`))
      (bind _output_get_4 (set `self.VOIPTalker_Ref` _returnvalue))
      (`/Engine/EditorBlueprintResources/StandardMacros.IsValid` _playerstate :!label _label
        (:`Is Valid`
          (`VOIPTalker.RegisterWithPlayerState` _output_get_4 _playerstate)
          (`VOIPStatics.SetMicThreshold` -1.0)
          (`/Engine/EditorBlueprintResources/StandardMacros.IsValid` _asbp_parent :!label _label_2
            (:`Is Valid`
              (set `VOIPTalker.Settings` (make `VoiceSettings` (`Character.CapsuleComponent` _asbp_parent) "/Game/Network/Core/SoundAtt_Microphone.SoundAtt_Microphone") (`self.VOIPTalker_Ref`)))
            (:`Is Not Valid`
              (`KismetSystemLibrary.Delay` 0.2)
              (goto _label_2))))
        (:`Is Not Valid`
          (`KismetSystemLibrary.Delay` 0.2)
          (goto _label))))))

(event `Client_SpawnPlayer`
  (bind _asgi_metaverse (cast `/Game/Network/Core/GI_Metaverse` (`GameplayStatics.GetGameInstance`)))
  (`self.Server_SpawningPlayer` (`/Game/Network/Core/GI_Metaverse.AvatarUrl` _asgi_metaverse)))

(event `Server_SpawningPlayer`
  (params (Url :type String))
  (bind _outactors (`GameplayStatics.GetAllActorsOfClass` "/Script/Engine.PlayerStart"))
  (for _array_element _outactors
    (if (!= (`PlayerStart.PlayerStartTag` _array_element) "X")
      (set `PlayerStart.PlayerStartTag` "X" _array_element)
      (break)))
  (bind _returnvalue (`|SpawnActorFromClass` "/Game/TestCharacters/ParentMain/BP_Parent.BP_Parent_C" (`self.GetTransform` _array_element) "Undefined" "OverrideRootScale" null null))
  (`/Game/TestCharacters/ParentMain/BP_Parent.LoadAvatarServer` _returnvalue Url)
  (bind _ascharacter (cast `Character` _returnvalue :!pure true))
  (`/Engine/EditorBlueprintResources/StandardMacros.IsValid` _ascharacter
    (:`Is Valid`
      (`CharacterMovementComponent.DisableMovement` (`Character.CharacterMovement` _ascharacter))
      (`self.Possess` _ascharacter))))

(event `OwingClient_KickPlayer`
  ;[1 1 1] Kick Player
  (`DestroySessionCallbackProxy.DestroySession` self
    (:`OnSuccess`
      (`GameplayStatics.OpenLevelBySoftObjectPtr` "/Game/Network/Map/Level_CharacterSelection.Level_CharacterSelection" true "listen"))))

(event `EndSessionByServer`
  ;[1 1 1] Host Destroy The Session (Used In Leave Session in WBP_MainUI)
  (`DestroySessionCallbackProxy.DestroySession` self
    (:`OnSuccess`
      (`GameplayStatics.OpenLevelBySoftObjectPtr` "/Game/Network/Map/Level_CharacterSelection.Level_CharacterSelection" true "listen"))))

(event `Server_SpawnPlayer`
  (params (Class :type "Actor Class Reference"))
  ;[1 1 1] Server
  (bind _outactors (`GameplayStatics.GetAllActorsOfClass` "/Script/Engine.PlayerStart"))
  (for _array_element _outactors
    (if (!= (`PlayerStart.PlayerStartTag` _array_element) "X")
      (set `PlayerStart.PlayerStartTag` "X" _array_element)
      (break)))
  (bind _returnvalue (`|SpawnActorFromClass` Class (`self.GetTransform` _array_element) "Undefined" "OverrideRootScale" null null))
  (bind _ascharacter (cast `Character` _returnvalue :!pure true))
  (`/Engine/EditorBlueprintResources/StandardMacros.IsValid` _ascharacter
    (:`Is Valid`
      (`CharacterMovementComponent.DisableMovement` (`Character.CharacterMovement` _ascharacter))
      (`self.Possess` _ascharacter)
      (`self.SetCamera`))))

(event `SetCamera`
  ;[1 1 1] Set Camera View
  (bind _outactors (`GameplayStatics.GetAllActorsOfClass` "/Script/Engine.CameraActor"))
  (for _array_element _outactors
    (bind _output_get (set `self.Camera_Ref` _array_element))
    (`self.SetViewTargetWithBlend` _output_get)))

(fn `UserConstructionScript`)