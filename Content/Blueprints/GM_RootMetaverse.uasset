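; Root game mode for the metaverse that starts GameLift hosting on the server and manages joining players.
; On server BeginPlay it hands itself to GI_Metaverse to initialize GameLift, and GameSessionStarted server-travels to the given map.
; PostLogin records each PC_Metaverse and triggers its client spawn call.
; Helpers respawn players as the game instance's character at a random PlayerStart or kick them by list index; SetCamera is empty.
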(event `self.ReceiveBeginPlay`
  ;[1 1 1] Initiate Connection to Gamelift
  (`parent.ReceiveBeginPlay`)
  (if (`KismetSystemLibrary.IsServer`)
    (bind _asgi_metaverse (cast `/Game/Network/Core/GI_Metaverse` (`GameplayStatics.GetGameInstance`)))
    (set `self.As GI Metaverse` _asgi_metaverse)
    (`/Game/Network/Core/GI_Metaverse.Init Gamelift` (`self.As GI Metaverse`) self)))

(event `self.K2_PostLogin`
  (params (NewPlayer :type "PlayerController Object Reference"))
  ;[1 1 1] When a player is connected (Must check all players)
  (set `self.New Player` NewPlayer)
  (bind _aspc_metaverse (cast `/Game/Network/Core/PC_Metaverse` NewPlayer))
  (set `self.PC Metaverse_Ref` _aspc_metaverse)
  (`|ExecutionSequence`
    (:`then_0`
      (`KismetArrayLibrary.Array_Add` (`self.AllPlayersController`) (`self.PC Metaverse_Ref`)))
    (:`then_1`
      (`/Game/Network/Core/PC_Metaverse.Client_SpawnPlayer` (`self.PC Metaverse_Ref`)))
    (:`then_2`
      (`self.SetCamera`))))

(event `self.K2_OnSwapPlayerControllers`
  (params (OldPC :type "PlayerController Object Reference") (NewPC :type "PlayerController Object Reference"))
  ;[1 1 1] When a player is connected (Must check all players)
  (`KismetArrayLibrary.Array_Add` (`self.JoinPlayers`) NewPC))

(event `GameSessionStarted`
  (params (Map :type String))
  (`KismetSystemLibrary.Delay` 0.0)
  (`KismetSystemLibrary.ExecuteConsoleCommand` (`KismetStringLibrary.Concat_StrStr` "servertravel" "/" Map) null))

(fn `Find_Random_PlayerStart`
  (returns (PlayerStartTransform :type "Transform Structure"))
  (bind _outactors (`GameplayStatics.GetAllActorsOfClass` "/Script/Engine.PlayerStart"))
  (return (`self.GetTransform` (`|GetArrayItem` _outactors (`KismetMathLibrary.RandomIntegerInRange` 0 (- (`KismetArrayLibrary.Array_Length` _outactors) 1))))))

(fn `KickPlayer`
  (params (PlayerID :type Integer))
  (`/Game/Network/Core/PC_Metaverse.OwingClient_KickPlayer` (`|GetArrayItem` (`self.AllPlayersController`) PlayerID)))

(fn `SetCamera`)

(fn `Spawn_Player`
  (params (PlayerController :type "PlayerController Object Reference"))
  (bind _returnvalue (`Controller.K2_GetPawn` PlayerController))
  (`/Engine/EditorBlueprintResources/StandardMacros.IsValid` _returnvalue
    (:`Is Valid`
      (`self.K2_DestroyActor` _returnvalue))
    (:`Is Not Valid`
      _))
  (bind _returnvalue_2 (`|SpawnActorFromClass` (`/Game/Network/Core/GI_Metaverse.Character` (cast `/Game/Network/Core/GI_Metaverse` (`GameplayStatics.GetGameInstance`) :!pure true)) (`self.Find_Random_PlayerStart`) "Undefined" "OverrideRootScale" null null))
  (`Controller.Possess` PlayerController _returnvalue_2))

(fn `UserConstructionScript`)