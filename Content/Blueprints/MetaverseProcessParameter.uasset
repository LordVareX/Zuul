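; MetaverseProcessParameter is a Blueprint handler for server process callbacks: game session start and update, termination and health checks, apparently for GameLift-style hosting.
; On session start, if the session name is empty, it reads the MAP game property into MapName and passes it to MetaverseGameMode's GameSessionStarted when that game mode is valid.
; Termination, session update and health check simply defer to the parent class.
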(event `self.ProcessTerminate`
  (`parent.ProcessTerminate`))

(event `self.StartGameSession`
  (params (gameSession :type "AWSGameSessionServer Structure"))
  (bind (_gamesessionid _name _fleetid _maximumplayersessioncount _status _gameproperties) (break `AWSGameSessionServer` gameSession))
  (bind _metaversegamemode (`self.MetaverseGameMode`))
  (if (`KismetStringLibrary.IsEmpty` _name)
    (for _array_element _gameproperties
      (bind (_key _value) (break `GamePropertyServer` _array_element))
      (if (`KismetStringLibrary.EqualEqual_StrStr` _key "MAP")
        (`KismetSystemLibrary.PrintString` null "Found")
        (set `self.MapName` _value)))
    (`/Engine/EditorBlueprintResources/StandardMacros.IsValid` _metaversegamemode
      (:`Is Valid`
        (`/Game/Network/Core/GM_Metaverse.GameSessionStarted` _metaversegamemode (`self.MapName`))))))

(event `self.UpdateGameSession`
  (params (updateGameSession :type "UpdateGameSessionServer Structure"))
  (`parent.UpdateGameSession` updateGameSession))

(fn `HealthCheck`
  (returns (ReturnValue :type Boolean))
  (bind _returnvalue (`parent.HealthCheck`))
  (return _returnvalue))